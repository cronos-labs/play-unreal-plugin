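; Example WalletConnect Blueprint that runs a Cronos Play wallet connection and transaction-signing demo on BeginPlay.
; After initializing the client, it registers a session callback, launches the connection URL on Android, and shows a QR code in WBP_WalletConnectUI if a BP_Cronos actor exists.
; A chain of async callbacks then ensures a session, signs a hard-coded legacy transaction, prints results and destroys the client after a short delay.
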(event `self.ReceiveBeginPlay`
  ;[1 1 1] InitializeWallet
  (`self.InitializeWalletConnect` "Defi WalletConnect example." "http://localhost:8080/" (`|MakeArray`) "Defi WalletConnect Web3 Example" (delegate `CustomEvent_InitializeWalletConnect`))
  (`KismetSystemLibrary.PrintString` "Initialize WalletConnect"))

(event `CustomEvent_SetupCallback`
  (params (SessionInfo :type "WalletConnectSessionInfo Structure"))
  (bind (_sessionstate _connected _accounts _chain_id) (break `WalletConnectSessionInfo` SessionInfo))
  ;[1 1 1] Setup Callback
  (`KismetSystemLibrary.PrintString` (`KismetStringLibrary.Concat_StrStr` "SessionInfo state=" (`|GetEnumeratorNameAsString` _sessionstate) "  chaind=" _chain_id "  connected=" (`KismetStringLibrary.Conv_BoolToString` _connected))))

(event `CustomEvent_EnsureSession`
  (params (SessionResult :type "WalletConnectEnsureSessionResult Structure") (Result :type String))
  (bind (_addresses _chain_id) (break `WalletConnectEnsureSessionResult` SessionResult))
  ;[1 1 1] EnsureSession
  (`KismetSystemLibrary.PrintString` (`KismetStringLibrary.Concat_StrStr` "EnsureSession OK=" Result "  chainid=" (`KismetTextLibrary.Conv_TextToString` (`KismetTextLibrary.Conv_Int64ToText` _chain_id))))
  ;[1 1 1] Sign TX
  (`self.SignLegacyTransactionBlocking` (make `WalletConnectTxLegacy` :`to` "0x0102030405010203040501020304050102030405" :`gas` "21000" :`gas_price` "10000" :`value` "100000000000000" :`nonce` "1") (`.address` (break `WalletConnectAddress` (`|GetArrayItem` _addresses))) (delegate `CustomEvent_0`))
  (`KismetSystemLibrary.PrintString` "Start Signing"))

(event `CustomEvent_InitializeWalletConnect`
  (params (Succeed :type Boolean) (message :type String))
  ;[1 1 1] InitializeWallet
  (if Succeed
    (`KismetSystemLibrary.PrintString` "Initialize WallectConnect OK")
    ;[1 1 1] Setup Callback
    (`self.SetupCallback` (delegate `CustomEvent_SetupCallback`))
    (`KismetSystemLibrary.PrintString` "Setup Callback")
    ;[1 1 1] Show QRCode
    (bind (_output _success) (`self.GetConnectionString`))
    (if (== (`GameplayStatics.GetPlatformName`) "Android")
      (`KismetSystemLibrary.LaunchURL` _output))
    (if _success
      (bind _outactors (`GameplayStatics.GetAllActorsOfClass` "/CronosPlayUnreal/CronosPlayUnreal/Blueprint/BP_Cronos.BP_Cronos_C"))
      (if (> (`KismetArrayLibrary.Array_Length` _outactors) 0)
        (bind _foundwidgets (`WidgetBlueprintLibrary.GetAllWidgetsOfClass` "/CronosPlayUnreal/CronosPlayUnreal/Blueprint/WBP_WalletConnectUI.WBP_WalletConnectUI_C"))
        (`/CronosPlayUnreal/CronosPlayUnreal/Blueprint/WBP_WalletConnectUI.SHOW_QRCODE` (`|GetArrayItem` _foundwidgets) _output)
        ;[1 1 1] EnsureSession
        (`self.EnsureSessionBlocking` (delegate `CustomEvent_EnsureSession`))
        (`KismetSystemLibrary.PrintString` "EnsureSession Start")))))

(event `CustomEvent_0`
  (params (SigningResult :type "WalletSignTXLegayResult Structure"))
  (bind (_signature _result) (break `WalletSignTXLegayResult` SigningResult))
  ;[1 1 1] Sign TX
  (`KismetSystemLibrary.PrintString` (`KismetStringLibrary.Concat_StrStr` "Signing Result Signature length=" (`KismetStringLibrary.Conv_IntToString` (`KismetArrayLibrary.Array_Length` _signature)) "  Result=" _result) true true (struct :`R` 1.0 :`A` 1.0) 60.0)
  (`KismetSystemLibrary.Delay` 1.0)
  (`self.DestroyClient`)
  (`KismetSystemLibrary.PrintString` "OK"))

(fn `UserConstructionScript`)