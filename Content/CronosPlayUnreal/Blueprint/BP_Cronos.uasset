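; Cronos Play blockchain actor that opens the demo page UI and sets up a wallet for the NFT screens.
; BeginPlay sets the SDK user agent and, if Showmenu is on, adds WBP_PageUI to the viewport.
; CustomEvent_Initialize, not called within this graph, loads a wallet from a hardcoded mnemonic with an empty password.
; On success it writes the first Ethereum address to the NFT and 1155 NFT widgets, where valid.
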(event `self.ReceiveBeginPlay`
  (`PlayCppSdkBPLibrary.SetupUserAgent` "CronosPlay-UnrealEngine-Agent")
  (if (`self.showmenu`)
    (bind _returnvalue (`|CreateWidget` "/CronosPlayUnreal/CronosPlayUnreal/Blueprint/WBP_PageUI.WBP_PageUI_C"))
    (`UserWidget.AddToViewport` _returnvalue 0)))

(event `CustomEvent_Initialize`
  (bind _mynft1155ui (`self.mynft1155ui`))
  (bind _mynftui (`self.mynftui`))
  ;[1 1 1] Initialize Wallet
  (bind (_output _success) (`self.InitializeWallet` "shed crumble dismiss loyal latin million oblige gesture shrug still oxygen custom remove ribbon disorder palace addict again blanket sad flock consider obey popular"))
  (if _success
    (`|ExecutionSequence`
      (:`then_0`
        ;[1 1 1] Print Eth Address
        (bind _output_2 (`self.GetEthAddress` 0))
        (if (`KismetSystemLibrary.IsValid` _mynftui)
          (`TextBlock.SetText` (`/CronosPlayUnreal/CronosPlayUnreal/Blueprint/WBP_NftErc721UI.TextBlock_WalletAddress` _mynftui) (`KismetTextLibrary.Conv_StringToText` _output_2))))
      (:`then_1`
        ;[1 1 1] Print Eth Address
        (bind _output_3 (`self.GetEthAddress` 0))
        (if (`KismetSystemLibrary.IsValid` _mynft1155ui)
          (`TextBlock.SetText` (`/CronosPlayUnreal/CronosPlayUnreal/Blueprint/WBP_NftErc1155UI1.TextBlock_WalletAddress` _mynft1155ui) (`KismetTextLibrary.Conv_StringToText` _output_3)))))))

(fn `UserConstructionScript`)